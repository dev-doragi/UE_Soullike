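; Enemy AI Blueprint that runs a behavior tree and feeds it pawn sightings.
; The behavior tree starts on BeginPlay.
; When PawnSensing sees a pawn, it writes a seen flag and the target actor to the Blackboard and mirrors both in local variables.
; It does no filtering of the sensed pawn and never clears the seen state.
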(event `self.ReceiveBeginPlay`
  (`self.RunBehaviorTree` (`self.Behavior Tree`)))

(event `self.PawnSensing.OnSeePawn`
  (params (Pawn :type "Pawn Object Reference"))
  (`BlackboardComponent.SetValueAsBool` (`AIBlueprintHelperLibrary.GetBlackboard` null) "seeingTarget?" true)
  (`BlackboardComponent.SetValueAsObject` (`AIBlueprintHelperLibrary.GetBlackboard` null) "targetActor" Pawn)
  (set `self.targetPawn` Pawn)
  (set `self.onSeePawn?` true))

(fn `UserConstructionScript`)