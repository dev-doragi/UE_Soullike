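; BP_WeaponPickable is a weapon pickup that takes its mesh from WeaponData at construction and gets an outline overlay material at BeginPlay.
; HighlightTrigger overlaps show or hide a widget, with timelines fading the outline through MPC_Outliner's Alpha, a collection parameter shared across instances.
; The Picked event plays a sound, then passes WeaponData to a BPI_Interact actor and destroys the pickup.
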(event `self.ReceiveBeginPlay`
  (`MeshComponent.SetOverlayMaterial` (`self.StaticMesh`) "/Game/Materials/MT_Outliner_Inst.MT_Outliner_Inst"))

(event `/Game/Blueprints/Weapons/BPI_Interact.Picked`
  (`GameplayStatics.PlaySoundAtLocation` "/Engine/VREditor/Sounds/UI/Object_PickUp.Object_PickUp" (`self.K2_GetActorLocation`) (struct) 3.0 1.0 0.0 "/Game/Audio/SA_Character.SA_Character" null null null)
  (if (`KismetSystemLibrary.DoesImplementInterface` (stale `self.Highlight Trigger.OnComponentBeginOverlap` OtherActor) "/Game/Blueprints/Weapons/BPI_Interact.BPI_Interact_C")
    (message `/Game/Blueprints/Weapons/BPI_Interact.Pickup Weapon` (stale `self.Highlight Trigger.OnComponentBeginOverlap` OtherActor) (`self.weaponData`))
    (`self.K2_DestroyActor`)))

(event `self.Highlight Trigger.OnComponentBeginOverlap`
  (params (OverlappedComponent :type "PrimitiveComponent Object Reference") (OtherActor :type "Actor Object Reference") (OtherComp :type "PrimitiveComponent Object Reference") (OtherBodyIndex :type Integer) (bFromSweep :type Boolean) (SweepResult :type "HitResult Structure (by ref)"))
  (if (`KismetSystemLibrary.DoesImplementInterface` OtherActor "/Game/Blueprints/Weapons/BPI_Interact.BPI_Interact_C")
    (`SceneComponent.SetVisibility` (`self.Widget`) true false)
    (bind (_direction _blendin) (`Timeline|BlendIn` :!via `PlayFromStart`)
      (:`Update`
        (`KismetMaterialLibrary.SetScalarParameterValue` "/Game/Materials/MPC_Outliner.MPC_Outliner" "Alpha" _blendin)))))

(event `self.Highlight Trigger.OnComponentEndOverlap`
  (params (OverlappedComponent :type "PrimitiveComponent Object Reference") (OtherActor :type "Actor Object Reference") (OtherComp :type "PrimitiveComponent Object Reference") (OtherBodyIndex :type Integer))
  (`SceneComponent.SetVisibility` (`self.Widget`) false false)
  (bind (_direction _blendin _blendout) (`Timeline|타임라인` :!via `PlayFromStart`)
    (:`Update`
      (`KismetMaterialLibrary.SetScalarParameterValue` "/Game/Materials/MPC_Outliner.MPC_Outliner" "Alpha" _blendout))))

(fn `UserConstructionScript`
  ;[1 1 1] Construct
  (`StaticMeshComponent.SetStaticMesh` (`self.StaticMesh`) (`/Game/Blueprints/Weapons/BP_DA_Weapon.staticMesh` (`self.weaponData`))))