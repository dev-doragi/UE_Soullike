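; Actor component that manages the third-person character's health and stamina and updates their progress bars.
; IncreaseValue clamps the chosen stat and refreshes its bar, sending DieMessage to the owner when health hits zero.
; A looping timer regenerates stamina outside dodges and attacks when allowed, at half rate while tired.
; Tick detects empty stamina, sets run speed and flags the character tired until a delay ends.
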(event `self.ReceiveBeginPlay`
  (bind _asbp_third_person_character (cast `/Game/ThirdPerson/Blueprints/BP_ThirdPersonCharacter` (`self.GetOwner`)))
  (set `self.PlayerBP` _asbp_third_person_character)
  (`KismetSystemLibrary.K2_SetTimerDelegate` (delegate `Regain Stamina`) 0.01 true))

(event `Regain Stamina`
  (bind _bpc_combats (`/Game/ThirdPerson/Blueprints/BP_ThirdPersonCharacter.BPC_Combats` (`self.PlayerBP`)))
  (if (and (`self.canRegainStamina?`) (not (`/Game/Blueprints/BPC_Combat.isDodging?` _bpc_combats)) (not (`/Game/Blueprints/BPC_Combat.isAttacking?` _bpc_combats)))
    (if (`self.isTired?`)
      (`self.Increase Value` "NewEnumerator1" 0.4)
      (else
        (`self.Increase Value` "NewEnumerator1" 0.8)))))

(event `Die`
  (message `/Game/Blueprints/BPI_Damage.Die` (`self.GetOwner`)))

(event `SetHealthProgressBar`
  (params (HealthProgressBar :type "ProgressBar Object Reference"))
  (set `self.healthProgressBar` HealthProgressBar))

(event `SetStaminaProgressBar`
  (params (staminaProgressBar :type "ProgressBar Object Reference"))
  (set `self.Stamina Progress Bar` staminaProgressBar))

(event `self.ReceiveTick`
  (params (DeltaSeconds :type "Float (single-precision)"))
  (bind _playerbp (`self.PlayerBP`))
  (if (<= (`self.currentStamina`) 0.0)
    (set `self.currentStamina` 0.0)
    (set `self.isTired?` true)
    (set `self.canRegainStamina?` true)
    (set `CharacterMovementComponent.MaxWalkSpeed` (`/Game/ThirdPerson/Blueprints/BP_ThirdPersonCharacter.RunSpeed` _playerbp) (`Character.CharacterMovement` _playerbp))
    (`KismetSystemLibrary.Delay` 2.0)
    (set `self.isTired?` false)))

(fn `Increase Value`
  (params (Stats :type "/Game/Blueprints/E_Stats Enum" :default "NewEnumerator0") (Value :type "Float (double-precision)"))
  (switch `/Game/Blueprints/E_Stats` Stats
    (:`NewEnumerator0`
      (set `self.currentHealth` (`KismetMathLibrary.FClamp` (+ (`self.currentHealth`) Value) 0.0 (`self.maxHealth`)))
      (`|ExecutionSequence`
        (:`then_0`
          (if (<= (`self.currentHealth`) 0.0)
            (`self.Die`)))
        (:`then_1`
          (bind _healthprogressbar (`self.healthProgressBar`)
            (:`then`
              (`ProgressBar.SetPercent` _healthprogressbar (/ (`self.currentHealth`) (`self.maxHealth`))))
            (:`else`)))))
    (:`NewEnumerator1`
      (set `self.currentStamina` (`KismetMathLibrary.FClamp` (+ (`self.currentStamina`) Value) 0.0 (`self.maxStamina`)))
      (`|ExecutionSequence`
        (:`then_1`
          (bind _stamina_progress_bar (`self.Stamina Progress Bar`)
            (:`then`
              (`ProgressBar.SetPercent` _stamina_progress_bar (/ (`self.currentStamina`) (`self.maxStamina`))))
            (:`else`)))))))